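; BP_Banana is a spinning banana actor that disappears when something overlaps it.
; Tick yaws it at a frame-rate-independent RotationSpeed.
; Overlap disables the mesh's collision and visibility, then a Delay leads into a DoOnce that restores both.
; The DoOnce is never reset, so the banana reappears only after the first overlap; a DestroyActor node is left unconnected.
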(event OnComponentBeginOverlap(StaticMesh)
  (params (OverlappedComponent :type Primitive%20Component%20Object%20Reference) (OtherActor :type Actor%20Object%20Reference) (OtherComp :type Primitive%20Component%20Object%20Reference) (OtherBodyIndex :type Integer) (bFromSweep :type Boolean) (SweepResult :type Hit%20Result%20Structure%20%28by%20ref%29))
  (bind _staticmesh (Variables|Default|GetStaticMesh))
  (bind _staticmesh_2 (Variables|Default|GetStaticMesh))
  (Collision|SetCollisionEnabled _staticmesh_2 "NoCollision")
  (Rendering|SetVisibility _staticmesh_2 false false)
  (Utilities|FlowControl|Delay 6.0)
  (Utilities|FlowControl|DoOnce false
    (:Completed
      (Collision|SetCollisionEnabled _staticmesh "QueryAndPhysics")
      (Rendering|SetVisibility _staticmesh true false))))

(event EventTick
  (params (DeltaSeconds :type Float%20%28single-precision%29))
  (Transformation|AddActorLocalRotation (Math|Rotator|MakeRotator 0.0 0.0 (* DeltaSeconds (Variables|Default|GetRotationSpeed))) false false))

(fn ConstructionScript)