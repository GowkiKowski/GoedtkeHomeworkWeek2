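; Player pawn for a banana collecting game, handling movement, sprinting, pickup counting and the win condition.
; Forward and right axis inputs feed movement input scaled by MaxSpeed, which Left Shift raises while held.
; Tick consumes that vector and applies it as a swept local offset, without using a movement component.
; Mesh overlaps with BP_Banana increment and print the total; reaching 30 prints a win message and quits after a delay.
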(event OnComponentBeginOverlap(CharacterMesh)
  (params (OverlappedComponent :type Primitive%20Component%20Object%20Reference) (OtherActor :type Actor%20Object%20Reference) (OtherComp :type Primitive%20Component%20Object%20Reference) (OtherBodyIndex :type Integer) (bFromSweep :type Boolean) (SweepResult :type Hit%20Result%20Structure%20%28by%20ref%29))
  (Utilities|Casting|CastToBP_Banana OtherActor)
  (Variables|Default|SetTotal%20Collected (+ (Variables|Default|GetTotal%20Collected) 1))
  (Development|PrintString (Utilities|String|ToString(Integer) (Variables|Default|GetTotal%20Collected)))
  (if (>= (Variables|Default|GetTotal%20Collected) 30)
    (Development|PrintString "Congratulations!")
    (Development|PrintString "You Win!!")
    (Utilities|FlowControl|Delay 2.0)
    (Game|QuitGame 0 "Quit" false)))

(event EventTick
  (params (DeltaSeconds :type Float%20%28single-precision%29))
  (bind _returnvalue (Class|Pawn|ConsumeMovementInputVector))
  (Transformation|AddActorLocalOffset (* _returnvalue DeltaSeconds) true false))

(event Input|AxisEvents|InputAxisMoveForwardBack
  (params (AxisValue :type Float%20%28single-precision%29))
  (Pawn|Input|AddMovementInput (Transformation|GetActorForwardVector) (* AxisValue (Variables|Default|GetMaxSpeed)) false))

(event Input|AxisEvents|InputAxisMoveRightLeft
  (params (AxisValue :type Float%20%28single-precision%29))
  (Pawn|Input|AddMovementInput (Transformation|GetActorRightVector) (* AxisValue (Variables|Default|GetMaxSpeed)) false))

(event Input|KeyboardEvents|LeftShift
  (params (Key :type Key%20Structure :default "None"))
  (:Pressed
    (Variables|Default|SetMaxSpeed 1.2e+03))
  (:Released
    (Variables|Default|SetMaxSpeed 6.5e+02)))

(fn ConstructionScript)